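; Development test actor that experiments with building geometry at runtime through a Procedural Mesh component.
; BeginPlay calls Voxel to fill the mesh buffers, then creates the section; the triangle and grid-quad builders are never called.
; Voxel adds eight cube corners but reuses the 11x11 grid triangle indices and leaves UVs empty, so the cube is unfinished.
; Normals and tangents come from CalculateTangentsForMesh.
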(event `self.ReceiveBeginPlay`
  (`self.Voxel`)
  (`ProceduralMeshComponent.CreateMeshSection_LinearColor` :`self` (`self.ProceduralMesh`) :`Vertices` (`self.Vertices`) :`Triangles` (`self.Triangles`) :`Normals` (`self.Normals`) :`UV0` (`self.UV`) :`Tangents` (`self.Tangents`)))

(fn `UserConstructionScript`)