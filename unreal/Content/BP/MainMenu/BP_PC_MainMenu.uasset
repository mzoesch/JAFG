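; BP_PC_MainMenu is the main menu player controller, exposing events that drive menu UI feedback.
; Events create and add a loading screen or error widget to the viewport, passing in the supplied text.
; Session search results are forwarded to the first top-level WBP_JoinSession widget found, if it is valid.
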(event `self.ShowLoadingScreen`
  (params (AdditionInformation :type "Text (by ref)"))
  (bind _returnvalue (`|CreateWidget` "/Game/Widgets/WBP_LoadingScreen.WBP_LoadingScreen_C" self AdditionInformation))
  (`UserWidget.AddToViewport` _returnvalue 0))

(event `self.ShowErrorMessage`
  (params (ErrorMessage :type "Text (by ref)"))
  (bind _returnvalue (`|CreateWidget` "/Game/Widgets/WBP_Error.WBP_Error_C" self ErrorMessage))
  (`UserWidget.AddToViewport` _returnvalue 0))

(event `self.OnSearchSessionsComplete`
  (params (SearchResults :type "Array of SearchResult Structure (by ref)"))
  (bind _foundwidgets (`WidgetBlueprintLibrary.GetAllWidgetsOfClass` "/Game/Widgets/MainMenu/WBP_JoinSession.WBP_JoinSession_C"))
  (bind _output (`|GetArrayItem` _foundwidgets))
  (`/Engine/EditorBlueprintResources/StandardMacros.IsValid` _output
    (:`Is Valid`
      (`/Game/Widgets/MainMenu/WBP_JoinSession.OnSearchSessionsComplete` _output SearchResults))))

(fn `UserConstructionScript`)